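; Interaction point actor for resolving a right thruster emergency.
; Its box overlap shows an instruction text while the emergency flag is active and hides it on exit.
; Interacting clears the flag, shows a restore text for two seconds, then notifies the first ExpandMenu widget found through GetAllWidgetsOfClass that the right thruster is resolved.
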(event `self.Box.OnComponentEndOverlap`
  (params (OverlappedComponent :type "PrimitiveComponent Object Reference") (OtherActor :type "Actor Object Reference") (OtherComp :type "PrimitiveComponent Object Reference") (OtherBodyIndex :type Integer))
  (`SceneComponent.SetVisibility` (`self.Instruction Text`) false false))

(event `self.Box.OnComponentBeginOverlap`
  (params (OverlappedComponent :type "PrimitiveComponent Object Reference") (OtherActor :type "Actor Object Reference") (OtherComp :type "PrimitiveComponent Object Reference") (OtherBodyIndex :type Integer) (bFromSweep :type Boolean) (SweepResult :type "HitResult Structure (by ref)"))
  (if (`self.RightThrusterEmergencyActive`)
    (`SceneComponent.SetVisibility` (`self.Instruction Text`) true false)))

(event `/Game/GlobalGameJam/Blueprints/Interaction/Interaction_Interface.Interact`
  (set `self.RightThrusterEmergencyActive` false)
  (`SceneComponent.SetVisibility` (`self.Instruction Text`) false false)
  (`SceneComponent.SetVisibility` (`self.Restore Text`) true false)
  (`KismetSystemLibrary.Delay` 2.0)
  (`SceneComponent.SetVisibility` (`self.Restore Text`) false false)
  (bind _foundwidgets (`WidgetBlueprintLibrary.GetAllWidgetsOfClass` "/Game/GlobalGameJam/Widget/ExpandMenu.ExpandMenu_C" false))
  (`/Game/GlobalGameJam/Widget/ExpandMenu.RightThruster Resolved` (`|GetArrayItem` _foundwidgets)))

(fn `UserConstructionScript`)