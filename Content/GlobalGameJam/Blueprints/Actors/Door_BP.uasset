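; A two-panel vertical door that moves when something enters or leaves its Box trigger.
; BeginPlay records both panels' starting world locations, and overlap resets each to it before timed MoveComponentTo calls drive the top up and the lower down.
; End overlap snaps each panel to the location saved during opening, then moves it toward the opposite fixed relative Z target.
; ZDistance-based offset math is left unconnected.
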(event `self.ReceiveBeginPlay`
  (set `self.Starting Top` (`SceneComponent.K2_GetComponentLocation` (`self.Door Top`)))
  (set `self.Starting Bottom` (`SceneComponent.K2_GetComponentLocation` (`self.Lower Door`))))

(event `self.Box.OnComponentBeginOverlap`
  (params (OverlappedComponent :type "PrimitiveComponent Object Reference") (OtherActor :type "Actor Object Reference") (OtherComp :type "PrimitiveComponent Object Reference") (OtherBodyIndex :type Integer) (bFromSweep :type Boolean) (SweepResult :type "HitResult Structure (by ref)"))
  (`SceneComponent.K2_SetWorldLocation` (`self.Door Top`) (`self.Starting Top`) false false)
  (`KismetSystemLibrary.MoveComponentTo` (`self.Door Top`) (0.0 0.0 250.0) (struct) false false 0.5)
  (set `self.FinishedTop` (`SceneComponent.K2_GetComponentLocation` (`self.Door Top`)))
  (`SceneComponent.K2_SetWorldLocation` (`self.Lower Door`) (`self.Starting Bottom`) false false)
  (`KismetSystemLibrary.MoveComponentTo` (`self.Lower Door`) (0.0 0.0 -250.0) (struct) false false 0.5)
  (set `self.Finished Bottom` (`SceneComponent.K2_GetComponentLocation` (`self.Lower Door`))))

(event `self.Box.OnComponentEndOverlap`
  (params (OverlappedComponent :type "PrimitiveComponent Object Reference") (OtherActor :type "Actor Object Reference") (OtherComp :type "PrimitiveComponent Object Reference") (OtherBodyIndex :type Integer))
  (`SceneComponent.K2_SetWorldLocation` (`self.Door Top`) (`self.FinishedTop`) false false)
  (`KismetSystemLibrary.MoveComponentTo` (`self.Door Top`) (0.0 0.0 -250.0) (struct) false false 0.5)
  (`SceneComponent.K2_SetWorldLocation` (`self.Lower Door`) (`self.Finished Bottom`) false false)
  (`KismetSystemLibrary.MoveComponentTo` (`self.Lower Door`) (0.0 0.0 250.0) (struct) false false 0.5))

(fn `UserConstructionScript`)