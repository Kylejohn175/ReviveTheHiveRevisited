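; RoomInteraction_BP is an interactable room station where the player fixes an electrical emergency on the ship.
; While the emergency flag is active, overlapping its box shows instruction text, which hides again on leaving.
; Interact clears the flag, briefly shows a restore message, then finds the ShipEvent_Actor and raises its ship-fix event with this room's type.
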(event `self.Box.OnComponentBeginOverlap`
  (params (OverlappedComponent :type "PrimitiveComponent Object Reference") (OtherActor :type "Actor Object Reference") (OtherComp :type "PrimitiveComponent Object Reference") (OtherBodyIndex :type Integer) (bFromSweep :type Boolean) (SweepResult :type "HitResult Structure (by ref)"))
  (if (`self.ElectricityEmergencyActive`)
    (`SceneComponent.SetVisibility` (`self.Instruction Text`) true false)))

(event `self.Box.OnComponentEndOverlap`
  (params (OverlappedComponent :type "PrimitiveComponent Object Reference") (OtherActor :type "Actor Object Reference") (OtherComp :type "PrimitiveComponent Object Reference") (OtherBodyIndex :type Integer))
  (`SceneComponent.SetVisibility` (`self.Instruction Text`) false false))

(event `/Game/GlobalGameJam/Blueprints/Interaction/Interaction_Interface.Interact`
  (set `self.ElectricityEmergencyActive` false)
  (`SceneComponent.SetVisibility` (`self.Instruction Text`) false false)
  (`SceneComponent.SetVisibility` (`self.Restore Text`) true false)
  (`KismetSystemLibrary.Delay` 2.0)
  (`SceneComponent.SetVisibility` (`self.Restore Text`) false false)
  ;[1 1 1] Event Handling
  (bind _returnvalue (`GameplayStatics.GetActorOfClass` "/Script/GlobalGameJam2020.ShipEvent_Actor"))
  (`ShipEvent_Actor.OnShipFixEvent` _returnvalue (`self.RoomType`)))

(fn `UserConstructionScript`)